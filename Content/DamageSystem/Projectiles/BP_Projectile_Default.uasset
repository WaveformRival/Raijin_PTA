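; BP_Projectile_Default is a damage-system projectile that flies at an optional Target, with configurable speed, gravity and homing.
; The construction script configures ProjectileMovement, enabling homing on the Target's root component when requested.
; With a valid Target, BeginPlay aims the velocity at it and ignores the instigator, or owner, during movement.
; On box hit, it calls OnProjectileHit, spawns Niagara, particle and sound impact effects, then destroys itself.
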(event `self.ReceiveBeginPlay`
  (bind _returnvalue (`self.GetInstigator`))
  (`self.Target`
    (:`then`
      (`self.RotateToTarget`)
      (`PrimitiveComponent.IgnoreActorWhenMoving` (`self.Box_Collision`) (select `bool` (`KismetSystemLibrary.IsValid` _returnvalue) :`false` (`self.GetOwner`) :`true` _returnvalue :!type "Actor Object Reference") true)
      (`PrimitiveComponent.IgnoreActorWhenMoving` (`self.StaticMesh`) (select `bool` (`KismetSystemLibrary.IsValid` _returnvalue) :`false` (`self.GetOwner`) :`true` _returnvalue :!type "Actor Object Reference") true))
    (:`else`)))

(event `RotateToTarget`
  (set `MovementComponent.Velocity` (* (`KismetMathLibrary.GetDirectionUnitVector` (`self.K2_GetActorLocation`) (`self.K2_GetActorLocation` (`self.Target`))) (`self.Speed`)) (`self.ProjectileMovement`)))

(event `self.Box_Collision.OnComponentHit`
  (params (HitComponent :type "PrimitiveComponent Object Reference") (OtherActor :type "Actor Object Reference") (OtherComp :type "PrimitiveComponent Object Reference") (NormalImpulse :type "Vector Structure") (Hit :type "HitResult Structure (by ref)"))
  (bind (_bblockinghit _binitialoverlap _time _distance _location) (`GameplayStatics.BreakHitResult` Hit))
  (`self.OnProjectileHit` OtherActor Hit)
  (`NiagaraFunctionLibrary.SpawnSystemAtLocation` (`self.ImpactEffect`) _location)
  (`GameplayStatics.SpawnEmitterAtLocation` (`self.ImpactPartical`) _location)
  (`GameplayStatics.SpawnSoundAtLocation` (`self.ImpactSound`) _location (struct) 1.0 1.0 0.0 null null)
  (`self.K2_DestroyActor`))

(fn `UserConstructionScript`
  (bind _projectilemovement (`self.ProjectileMovement`))
  (set `ProjectileMovementComponent.InitialSpeed` (`self.Speed`) _projectilemovement)
  (set `ProjectileMovementComponent.MaxSpeed` (`self.Speed`) _projectilemovement)
  (set `ProjectileMovementComponent.ProjectileGravityScale` (`self.Gravity`) _projectilemovement)
  (`self.Target`
    (:`then`
      (if (`self.IsHomi?`)
        (set `ProjectileMovementComponent.bIsHomingProjectile` true _projectilemovement)
        (set `ProjectileMovementComponent.HomingTargetComponent` (`Actor.RootComponent` (`self.Target`)) _projectilemovement)
        (set `ProjectileMovementComponent.bRotationFollowsVelocity` true _projectilemovement)))
    (:`else`)))