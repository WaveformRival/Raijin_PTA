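; Damage system component that tracks an actor's health and death, with functions to heal and take damage.
; TakeDamage routes a damage info struct through CanBeDamaged, which weighs death, invincibility and blocking to block, apply or ignore the hit.
; Outcomes fire blocked, death or damage response events, though the interruptible check currently changes nothing.
; Heal clamps health between zero and maximum while alive.
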(fn `Heal`
  (params (HealAmount :type "Float (double-precision)"))
  (returns (NewHealth :type "Float (double-precision)"))
  (if (not (`self.IsDead?`))
    (bind _output_get (set `self.CurrentHealth` (`KismetMathLibrary.FClamp` (+ HealAmount (`self.CurrentHealth`)) 0.0 (`self.MaxHealth`))))
    (return _output_get)))

(fn `TakeDamage`
  (params (DamageInfo :type "/Game/All_GameData/DamageSystem/S_DamageInfo Structure"))
  (returns (WasDamaged :type Boolean))
  (bind (_amount _damagetype _damageresponce _candamageinvicible _canbeblock _canbeparried _shouldbeinteract) (break `/Game/All_GameData/DamageSystem/S_DamageInfo` DamageInfo))
  (`self.CanBeDamaged` _candamageinvicible _canbeblock
    (:`BlockDamage`
      (`self.OnBlocked` _canbeparried)
      (return false))
    (:`DoDamage`
      (bind _output_get (set `self.CurrentHealth` (- (`self.CurrentHealth`) _amount)))
      (if (<= _output_get 0.0)
        (set `self.IsDead?` true)
        (`self.OnDeath`)
        (else
          (if (or (`self.InInterruptible?`) _shouldbeinteract)
            _
            (else
              _))
          (`self.OnDamageResponse` _damageresponce)))
      (return true))
    (:`NoDamage`
      (return false))))